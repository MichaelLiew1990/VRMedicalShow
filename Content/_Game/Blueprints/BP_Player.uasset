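; VR player Blueprint for Vive: a right-hand laser pointer that clicks widgets and manipulates a rotatable display platform.
; Trigger press caches hand pose and hit point, then uses component tags to select rotate or scale.
; Tick trims the laser to its trace, yaws the platform by sideways hand offset, and scales its contents or current sub-mesh by clamped, cubed radial drag.
; A timeline animates the left pad UI open and closed.
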(event Custom|HidePadUI
  (bind _padbroad (Variables|Default|GetPadBroad))
  (bind _padbroad_2 (Variables|Default|GetPadBroad))
  (bind _returnvalue (Transformation|GetWorldScale _padbroad))
  (bind (_x _y _z) (Math|Vector|BreakVector _returnvalue))
  ;[1 1 1] 动画显示/隐藏Pad
  (bind _padheight (Timeline|ShowPad ReverseFromEnd)
    (:Update
      (Class|WidgetComponent|SetDrawSize (Variables|Default|GetWidgetLeft) (Math|Vector2D|MakeVector2D 4e+02 (* _padheight 5e+02)))
      (Transformation|SetRelativeScale3D _padbroad_2 (Math|Vector|MakeVector (* _padheight 2.5) _y _z)))
    (:Finished
      (if (< _padheight 0.0001)
        (Rendering|SetVisibility _padbroad_2 false true)))))

(event Custom|ShowPadUI
  (bind _padbroad (Variables|Default|GetPadBroad))
  (bind _padbroad_2 (Variables|Default|GetPadBroad))
  (bind _returnvalue (Transformation|GetWorldScale _padbroad))
  (bind (_x _y _z) (Math|Vector|BreakVector _returnvalue))
  ;[1 1 1] 动画显示/隐藏Pad
  (Rendering|SetVisibility _padbroad true true)
  (bind _padheight (Timeline|ShowPad PlayFromStart)
    (:Update
      (Class|WidgetComponent|SetDrawSize (Variables|Default|GetWidgetLeft) (Math|Vector2D|MakeVector2D 4e+02 (* _padheight 5e+02)))
      (Transformation|SetRelativeScale3D _padbroad_2 (Math|Vector|MakeVector (* _padheight 2.5) _y _z)))
    (:Finished
      (if (< _padheight 0.0001)
        (Rendering|SetVisibility _padbroad_2 false true)))))

(event Custom|ViveTriggerPressed%28R%29
  (bind _rightforwardarrow (Variables|Default|GetRightForwardArrow))
  ;[1 1 1] 扳机触发UI点击事件
  (Class|WidgetInteractionComponent|PressPointerKey (Variables|Default|GetWidgetInteraction) "LeftMouseButton")
  (Variables|Default|SetIsRightTiggerPressed true)
  (Variables|Default|SetOrginArrowLoc (Transformation|GetWorldLocation _rightforwardarrow))
  (Variables|Default|SetOrginArrowDir (Math|Vector|GetForwardVector _rightforwardarrow))
  (Variables|Default|SetOrginYaw (.Yaw (CallFunction|GetPlatformRotator)))
  (bind (_impactpoint _hitcomponent _ishit) (CallFunction|GetLineHit))
  (if _ishit
    (Variables|Default|SetOrginImpactToCenterLength (Math|Vector|VectorLength (- _impactpoint (Transformation|GetWorldLocation (Variables|/Game/_Game/Blueprints/BP_RotatePlatform.BP_RotatePlatform_C|Getroot (Variables|Setup|GetRotatePlatform))))))
    (Utilities|FlowControl|Sequence
      (:then_0
        (if (Components|ComponentHasTag _hitcomponent "PlatformRotation")
          (Variables|Default|SetCanRotatePlatform true)
          (elif (Components|ComponentHasTag _hitcomponent "PlatformScale")
            (Variables|Default|SetCanScalePlatform true))))
      (:then_1
        (Variables|Default|SetLastScale (.X (Math|Vector|BreakVector (Variables|/Script/Engine.SceneComponent|GetRelativeScale3D (Variables|/Game/_Game/Blueprints/BP_RotatePlatform.BP_RotatePlatform_C|GetPlatformScale (Variables|Setup|GetRotatePlatform))))))
        (bind _normal (CallFunction|GetScaleNomal _impactpoint))
        (Variables|Default|SetPlatformScaleNormal _normal)))))

(event Custom|ViveTriggerRelease%28R%29
  ;[1 1 1] 扳机触发UI点击事件
  (Class|WidgetInteractionComponent|ReleasePointerKey (Variables|Default|GetWidgetInteraction) "LeftMouseButton")
  (Variables|Default|SetIsRightTiggerPressed false)
  (Variables|Default|SetCanRotatePlatform false)
  (Variables|Default|SetCanScalePlatform false))

(event EventTick
  (params (DeltaSeconds :type Float%20%28single-precision%29))
  (bind (_canscale _scalevalue) (CallFunction|GetPlatformScale))
  (bind _orginarrowloc (Variables|Default|GetOrginArrowLoc))
  (bind _orginarrowdir (Variables|Default|GetOrginArrowDir))
  (bind _raserline (Variables|Default|GetRaserLine))
  (bind _rightforwardarrow (Variables|Default|GetRightForwardArrow))
  (bind _returnvalue (Math|Float|Power _scalevalue 3.0))
  (bind _returnvalue_2 (Transformation|GetWorldLocation _rightforwardarrow))
  (bind _returnvalue_3 (* _orginarrowdir 1e+02))
  (bind _returnvalue_4 (+ _orginarrowloc "0, 0,100.000000"))
  (bind _returnvalue_5 (Math|Float|Sqrt _returnvalue))
  (bind _returnvalue_6 (+ _orginarrowloc _returnvalue_3))
  (bind _v (CallFunction|GetDistancetoPlanebyPointPure _returnvalue_2 _orginarrowloc _returnvalue_6 _returnvalue_4))
  (bind _returnvalue_7 (Math|Float|Sqrt _returnvalue_5))
  ;[1 1 1] 绘制激光射线
  (Utilities|FlowControl|Sequence
    (:then_0
      (bind (_impactpoint _hitcomponent _ishit) (CallFunction|GetLineHit))
      (if _ishit
        (Utilities|FlowControl|Sequence
          (:then_0
            (SplineMesh|SetEndPosition _raserline (Math|Vector|MakeVector (Math|Vector|VectorLength (- _impactpoint (Transformation|GetWorldLocation (Variables|Default|GetRightHandArrow)))) 0.0 0.0) true))
          (:then_1
            (Variables|Default|SetImpactPoint _impactpoint)))
        (else
          (SplineMesh|SetEndPosition _raserline "1000.000000, 0, 0" true))))
    (:then_1
      (if (Variables|Default|GetCanRotatePlatform)
        ;;[1 1 1] 底座旋转
        (if (> (.Z (Math|Vector|BreakVector (Math|Vector|CrossProduct (- _returnvalue_2 _orginarrowloc) _orginarrowdir))) 0.0)
          (Variables|Default|SetCurrentPlatformRotator (.Rotator (Utilities|MakeCurrentRotator (* _v 0.1))))
          (else
            (Variables|Default|SetCurrentPlatformRotator (.Rotator (Utilities|MakeCurrentRotator (* _v -0.1))))))
        (Transformation|SetWorldRotation (Variables|/Game/_Game/Blueprints/BP_RotatePlatform.BP_RotatePlatform_C|Getroot (Variables|Setup|GetRotatePlatform)) (Variables|Default|GetCurrentPlatformRotator) false false)))
    (:then_2
      ;;[1 1 1] 底座缩放
      (if _canscale
        (Variables|Default|SetCurPlatformStuffScale (Math|Vector|MakeVector _returnvalue _returnvalue _returnvalue))
        (if (Variables|Default|GetIsScaleSubSystem)
          (Transformation|SetRelativeScale3D (Variables|/Game/_Game/Blueprints/BP_StuffManager.BP_StuffManager_C|GetCurrentSubMeshComp (Variables|Setup|GetStuffManager)) (Variables|Default|GetCurPlatformStuffScale))
          (else
            (Transformation|SetRelativeScale3D (Variables|/Game/_Game/Blueprints/BP_RotatePlatform.BP_RotatePlatform_C|GetStuff (Variables|Setup|GetRotatePlatform)) (Variables|Default|GetCurPlatformStuffScale))))
        (Transformation|SetRelativeScale3D (Variables|/Game/_Game/Blueprints/BP_RotatePlatform.BP_RotatePlatform_C|GetPlatformScale (Variables|Setup|GetRotatePlatform)) (Math|Vector|MakeVector _returnvalue_7 _returnvalue_7 1.0))))))

(fn ConstructionScript)

(fn GetPlatformRotator
  (bind _rotateplatform (Variables|Setup|GetRotatePlatform))
  (bind _root (Variables|/Game/_Game/Blueprints/BP_RotatePlatform.BP_RotatePlatform_C|Getroot _rotateplatform))
  (bind _returnvalue (Transformation|GetWorldRotation _root))
  (return _returnvalue (.Yaw (Math|Rotator|BreakRotator _returnvalue))))

(fn GetLineHit
  (bind _righthandarrow (Variables|Default|GetRightHandArrow))
  (bind _returnvalue (Transformation|GetWorldLocation _righthandarrow))
  (bind (_outhit _returnvalue_2) (Collision|LineTraceByChannel _returnvalue (+ _returnvalue (* (Math|Vector|GetForwardVector _righthandarrow) 1e+03)) "TraceTypeQuery1" false 0 "None" false))
  (return (.ImpactPoint (Collision|BreakHitResult _outhit)) (.HitComponent (Collision|BreakHitResult _outhit)) _returnvalue_2))

(fn GetScaleNomal
  (params (ImpactPoint :type Vector))
  (bind _rotateplatform (Variables|Setup|GetRotatePlatform))
  (bind _root (Variables|/Game/_Game/Blueprints/BP_RotatePlatform.BP_RotatePlatform_C|Getroot _rotateplatform))
  (bind _returnvalue (Transformation|GetWorldLocation _root))
  (return (Math|Vector|CrossProduct (+ _returnvalue (* (Math|Vector|GetUpVector _root) 1e+01)) (- ImpactPoint _returnvalue))))

(fn GetPlatformScale
  (bind _impactpoint (Variables|Default|GetImpactPoint))
  (bind _rotateplatform (Variables|Setup|GetRotatePlatform))
  (bind _root (Variables|/Game/_Game/Blueprints/BP_RotatePlatform.BP_RotatePlatform_C|Getroot _rotateplatform))
  (bind _returnvalue (Transformation|GetWorldLocation _root))
  (bind _returnvalue_2 (- _impactpoint _returnvalue))
  (if (Variables|Default|GetCanScalePlatform)
    (LocalVariables|SetReValue (Math|Float|Clamp(Float) (* (/ (Math|Vector|VectorLength _returnvalue_2) (Variables|Default|GetOrginImpactToCenterLength)) (Variables|Default|GetLastScale)) 0.75 1.5))
    (LocalVariables|SetReBool (and (> (.Z (Math|Vector|BreakVector (Math|Vector|CrossProduct _returnvalue_2 (Variables|Default|GetPlatformScaleNormal)))) 0.0) (Variables|Default|GetCanScalePlatform)))
    (else
      (LocalVariables|SetReValue 1.0)
      (LocalVariables|SetReBool false)))
  (return (LocalVariables|GetReBool) (LocalVariables|GetReValue)))