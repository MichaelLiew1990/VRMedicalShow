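; BP_ManBase is a base actor for a man that can move itself onto a rotating platform and attach to it.
; On BeginPlay it caches the first BP_RotatePlatform found in the level.
; AttachToPlatform tweens position and rotation to the platform's Stuff component over one second, then, after a matching delay, snap-attaches to that component.
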(event Custom|AttachToPlatform
  (bind _platform (Variables|Default|GetPlatform))
  (bind _root (Variables|Default|Getroot))
  (bind _stuff (Variables|/Game/_Game/Blueprints/BP_RotatePlatform.BP_RotatePlatform_C|GetStuff _platform))
  (Class|ITween|ActorMovefromtoSimple "No Name" self (Transformation|GetWorldLocation _root) (Transformation|GetWorldLocation _stuff) "world" false 1.0 "linear")
  (Class|ITween|ActorRotatefromtoSimple "No Name" self (Transformation|GetWorldRotation _root) (Transformation|GetWorldRotation _stuff) "world" false 1.0 "linear")
  (Utilities|FlowControl|Delay 1.0)
  (Transformation|AttachComponentToComponent (Variables|/Game/_Game/Blueprints/BP_RotatePlatform.BP_RotatePlatform_C|GetStuff (Variables|Default|GetPlatform)) "None" "SnapToTarget" "SnapToTarget" "SnapToTarget" true))

(event EventBeginPlay
  (bind _outactors (Actor|GetAllActorsOfClass "/Game/_Game/Blueprints/BP_RotatePlatform.BP_RotatePlatform_C"))
  (Variables|Default|SetPlatform (Utilities|Array|Get(acopy) _outactors)))

(fn ConstructionScript)