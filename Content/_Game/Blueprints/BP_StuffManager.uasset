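; Manager actor for an anatomy display that separates eight body systems, such as skeleton, muscle and viscera, or combines them.
; BeginPlay fills two index-matched arrays of part components and their target billboards.
; Separare tweens each part's world location and rotation to its own billboard, while Combine tweens all parts to one shared billboard.
; Named tweens let each action stop the opposite one before starting from the current transforms.
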(event Custom|Combine
  (|CombineAllParts))

(event Custom|Separare
  (|SeparateAllParts))

(event EventBeginPlay
  (|InitialAllParts))

(fn ConstructionScript)